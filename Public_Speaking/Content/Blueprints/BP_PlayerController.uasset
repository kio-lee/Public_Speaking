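; BP_PlayerController is a player controller that maps keyboard keys to manual controls for an LLM-driven group NPC conversation in VR.
; Left, Down and Right force Cooper, Danielle or Lena to ask a question through the BP_Group_NPC_LLM actor, which is found lazily and cached.
; Enter and Backspace start and stop speech collection on the VRPawn.
; Right Shift tells VRGameMode to save to file.
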(event `Key|Left`
  (params (Key :type "Key Structure"))
  (:`Pressed`
    (bind _llm_ref (`self.Get gorup ref`))
    (`/Game/Demo/LLM/BP_Group_NPC_LLM.ForceTargetCharacterToAskQuestion` _llm_ref "Cooper")))

(event `Key|Up`
  (params (Key :type "Key Structure")))

(event `Key|Down`
  (params (Key :type "Key Structure"))
  (:`Pressed`
    (bind _llm_ref (`self.Get gorup ref`))
    (`/Game/Demo/LLM/BP_Group_NPC_LLM.ForceTargetCharacterToAskQuestion` _llm_ref "Danielle")))

(event `Key|Right`
  (params (Key :type "Key Structure"))
  (:`Pressed`
    (bind _llm_ref (`self.Get gorup ref`))
    (`/Game/Demo/LLM/BP_Group_NPC_LLM.ForceTargetCharacterToAskQuestion` _llm_ref "Lena")))

(event `Key|Enter`
  (params (Key :type "Key Structure"))
  (:`Pressed`
    (bind _returnvalue (`GameplayStatics.GetActorOfClass` "/Game/VRTemplate/Blueprints/VRPawn.VRPawn_C"))
    (if (`KismetSystemLibrary.IsValid` _returnvalue)
      (`/Game/VRTemplate/Blueprints/VRPawn.CollectSpeach` _returnvalue)
      (else
        (`KismetSystemLibrary.PrintString` "Invalid VRPAwn")))))

(event `Key|BackSpace`
  (params (Key :type "Key Structure"))
  (:`Pressed`
    (bind _returnvalue (`GameplayStatics.GetActorOfClass` "/Game/VRTemplate/Blueprints/VRPawn.VRPawn_C"))
    (if (`KismetSystemLibrary.IsValid` _returnvalue)
      (`/Game/VRTemplate/Blueprints/VRPawn.StopGatheringSpeach` _returnvalue)
      (else
        (`KismetSystemLibrary.PrintString` "Invalid VRPAwn")))))

(event `Key|RightShift`
  (params (Key :type "Key Structure"))
  (:`Pressed`
    (bind _asvrgame_mode (cast `/Game/VRTemplate/Blueprints/VRGameMode` (`GameplayStatics.GetGameMode`)))
    (`LoggerGameMode.SaveFileToFile` _asvrgame_mode)))

(fn `Get gorup ref`
  (returns (`LLM ref` :type "/Game/Demo/LLM/BP_Group_NPC_LLM Object Reference"))
  (`/Engine/EditorBlueprintResources/StandardMacros.IsValid` (`self.GroupNpc`)
    (:`Is Valid`
      (return (`self.GroupNpc`)))
    (:`Is Not Valid`
      (bind _returnvalue (`GameplayStatics.GetActorOfClass` "/Game/Demo/LLM/BP_Group_NPC_LLM.BP_Group_NPC_LLM_C"))
      (bind _output_get (set `self.GroupNpc` _returnvalue))
      (return _output_get))))

(fn `UserConstructionScript`)